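; Game mode Blueprint that keeps the game's score, with separate point values for goodies and baddies.
; BeginPlay resets the score and sets both values, with the goodie value larger than the baddie value.
; SumarPuntos adds the baddie value and RestarPuntos subtracts the goodie value.
; Each score change, like the initial reset, prints the score as a debug string.
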(event Custom|SumarPuntos
  (Variables|Default|SetScore (+ (Variables|Default|GetScore) (Variables|Default|GetPuntaje%20Baddie)))
  (Development|PrintString (Utilities|String|ToString(Integer) (Variables|Default|GetScore))))

(event Custom|RestarPuntos
  (Variables|Default|SetScore (- (Variables|Default|GetScore) (Variables|Default|GetPuntaje%20Goodie)))
  (Development|PrintString (Utilities|String|ToString(Integer) (Variables|Default|GetScore))))

(event EventBeginPlay
  (Variables|Default|SetScore 0)
  (Variables|Default|SetPuntaje%20Goodie 300)
  (Variables|Default|SetPuntaje%20Baddie 100)
  (Development|PrintString (Utilities|String|ToString(Integer) (Variables|Default|GetScore))))

(event EventTick
  (params (DeltaSeconds :type Float%20%28single-precision%29)))

(fn ConstructionScript)