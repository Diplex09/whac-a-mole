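; Whack-a-mole hole actor that repeatedly pops up either a good or a bad mole after a random delay, with bad more likely.
; The ArribaAbajo timeline raises the chosen mesh, then reverses after a random hittable window, and its Finished event restarts the cycle once hidden.
; EventoTopoGolpeado recolors TopoBueno's dynamic material, closes the hit window and immediately lowers the mole only if it is good.
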(event Custom|EventoBajar
  ;[1 1 1] Loop para subir o bajar al Topo bueno
  (bind _z_topo (Timeline|ArribaAbajo ReverseFromEnd)
    (:Update
      (Transformation|SetRelativeLocation (Variables|Default|GetTopo%20a%20levantar) (Math|Vector|MakeVector 0.0 1e+02 _z_topo) false false))
    (:Finished
      (if (Variables|Default|GetEscondido?)
        (Variables|Default|SetEscondido? false)
        (Variables|Default|SetCollisionable? true)
        (Utilities|FlowControl|Delay (Math|Random|RandomFloatinRange 0.0 1.0))
        (if (Variables|Default|GetCollisionable?)
          (Variables|Default|SetCollisionable? false)
          (CallFunction|EventoBajar))
        (else
          (Variables|Default|SetEscondido? true)
          (CallFunction|EventoSubir))))))

(event Custom|EventoSubir
  (if (Variables|Default|GetGolpeado?)
    (Variables|Default|SetGolpeado? false)
    (Rendering|Material|SetVectorParameterValue (Variables|Default|GetTopo_Mat) "color" (Variables|Default|GetColor_Topo_Original) :!class /Script/Engine.MaterialInstanceDynamic))
  (Utilities|FlowControl|Delay (Math|Random|RandomFloatinRange 2.0 4.0))
  (Math|Integer|CompareInt (Math|Random|RandomIntegerinRange 1 4) 1
    (:>
      (Variables|Default|SetGoodie? false)
      (Variables|Default|SetTopo%20a%20levantar (Variables|Default|GetTopo%20Malo))
      ;[1 1 1] Loop para subir o bajar al Topo bueno
      (bind _z_topo (Timeline|ArribaAbajo PlayFromStart)
        (:Update
          (Transformation|SetRelativeLocation (Variables|Default|GetTopo%20a%20levantar) (Math|Vector|MakeVector 0.0 1e+02 _z_topo) false false))
        (:Finished
          (if (Variables|Default|GetEscondido?)
            (Variables|Default|SetEscondido? false)
            (Variables|Default|SetCollisionable? true)
            (Utilities|FlowControl|Delay (Math|Random|RandomFloatinRange 0.0 1.0))
            (if (Variables|Default|GetCollisionable?)
              (Variables|Default|SetCollisionable? false)
              (CallFunction|EventoBajar))
            (else
              (Variables|Default|SetEscondido? true)
              (CallFunction|EventoSubir))))))
    (:==
      (Variables|Default|SetGoodie? true)
      (Variables|Default|SetTopo%20a%20levantar (Variables|Default|GetTopo%20Bueno))
      (Timeline|ArribaAbajo PlayFromStart))))

(event Custom|Evento%20Topo%20Golpeado
  ;[1 1 1] Cuando el martillo coliciona con el topo
  (if (Variables|Default|GetCollisionable?)
    (Variables|Default|SetCollisionable? false)
    (Development|PrintString "Topo golpeado")
    (Rendering|Material|SetVectorParameterValue (Variables|Default|GetTopo_Mat) "color" (Variables|Default|GetColor_Topo_Golpeado) :!class /Script/Engine.MaterialInstanceDynamic)
    (Variables|Default|SetGolpeado? true)
    (if (Variables|Default|GetGoodie?)
      (CallFunction|EventoBajar))))

(event EventBeginPlay
  (CallFunction|EventoSubir))

(fn ConstructionScript
  (bind _topo_bueno (Variables|Default|GetTopo%20Bueno))
  (bind _returnvalue (Rendering|Material|CreateDynamicMaterialInstance _topo_bueno 0 (Rendering|Material|GetMaterial _topo_bueno 0) "" :!class /Script/Engine.PrimitiveComponent))
  (bind _output_get (Variables|Default|SetTopo_Mat _returnvalue))
  (Rendering|Material|SetVectorParameterValue _output_get "color" (Variables|Default|GetColor_Topo_Original) :!class /Script/Engine.MaterialInstanceDynamic))