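; Hammer actor for a whack-a-mole game that swings on left mouse click and scores hits on moles (Topo_BP).
; A click, throttled by a DoOnce with a short delay, plays the GolpeMartillo timeline to rotate the root, and a FlipFlop on Finished reverses it to raise the hammer.
; HammerCollision overlaps subtract points in GameMode_BP for Goodie moles, add them for others, and notify the struck mole.
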(event OnComponentBeginOverlap(HammerCollision)
  (params (OverlappedComponent :type Primitive%20Component%20Object%20Reference) (OtherActor :type Actor%20Object%20Reference) (OtherComp :type Primitive%20Component%20Object%20Reference) (OtherBodyIndex :type Integer) (bFromSweep :type Boolean) (SweepResult :type Hit%20Result%20Structure%20%28by%20ref%29))
  (bind _as_game_mode_bp (Variables|Default|GetAs%20Game%20Mode%20BP))
  (bind _astopo_bp (Utilities|Casting|CastToTopo_BP OtherActor))
  (if (Variables|/Game/BP/Topo_BP.Topo_BP_C|GetGoodie? _astopo_bp)
    (Default|RestarPuntos _as_game_mode_bp)
    (else
      (Default|SumarPuntos _as_game_mode_bp)))
  (Default|EventoTopoGolpeado _astopo_bp)
  (Development|PrintString "Martillo chocó"))

(event Custom|EventoSubir
  (bind _x_hammer (Timeline|GolpeMartillo ReverseFromEnd)
    (:Update
      (Transformation|SetRelativeRotation (Variables|Default|GetDefaultSceneRoot) (Math|Rotator|MakeRotator _x_hammer 0.0 0.0) false false))
    (:Finished
      (Utilities|FlowControl|FlipFlop
        (:A
          (CallFunction|EventoSubir))))))

(event Custom|EventoBajar
  (bind _x_hammer (Timeline|GolpeMartillo Play)
    (:Update
      (Transformation|SetRelativeRotation (Variables|Default|GetDefaultSceneRoot) (Math|Rotator|MakeRotator _x_hammer 0.0 0.0) false false))
    (:Finished
      (Utilities|FlowControl|FlipFlop
        (:A
          (CallFunction|EventoSubir))))))

(event EventBeginPlay
  (bind _asgame_mode_bp (Utilities|Casting|CastToGameMode_BP (Game|GetGameMode)))
  (Variables|Default|SetAs%20Game%20Mode%20BP _asgame_mode_bp))

(event Input|MouseEvents|LeftMouseButton
  (params (Key :type Key%20Structure :default "None"))
  (:Pressed
    (Utilities|FlowControl|DoOnce false :!label _label
      (:Completed
        (CallFunction|EventoBajar)
        (Utilities|FlowControl|Delay 0.3)
        (goto _label Reset)))))

(event Input|MouseEvents|Mouse2D
  (params (AxisValue :type Vector :default "0, 0, 0")))

(fn ConstructionScript)