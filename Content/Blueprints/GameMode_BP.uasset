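; Game mode for a timed hammer game that keeps score, penalizing goodie hits and rewarding baddie points, and runs a countdown.
; BeginPlay creates the HUD, starts music and caches the hammer actor.
; Tick drives the countdown through a one-second Delay, advancing the HUD progress bar until TimeOut disables the hammer, swaps audio and shows game over.
; A count-up timer and an older score-refresh event remain, the former unused.
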(event Custom|SumarPuntos
  ;[1 1 1] Actualizar puntaje
  (Variables|Default|SetScore (+ (Variables|Default|GetScore) (Variables|Default|GetPuntaje%20Baddie))))

(event Custom|RestarPuntos
  ;[1 1 1] Actualizar puntaje
  (Variables|Default|SetScore (- (Variables|Default|GetScore) (Variables|Default|GetPuntaje%20Goodie))))

(event Custom|ImprimirPuntajeActual
  ;[1 1 1] Imprimir puntaje antiguo, antes de la función binding en Hud_BP
  (Default|ActualizarScore (Variables|Default|GetScoreUI) (Variables|Default|GetScore)))

(event Custom|ContarTiempo
  ;[1 1 1] Para emular un cronómetro
  (Utilities|FlowControl|Delay 1.0)
  (Math|Integer|CompareInt (Variables|Default|GetSeconds) 59
    (:==
      (Math|Integer|IncrementInt (Variables|Default|GetMinutes)
        (:%20%20
          (Variables|Default|SetSeconds 0))))
    (:<
      (Math|Integer|IncrementInt (Variables|Default|GetSeconds)))))

(event Custom|CuentaRegresiva
  ;[1 1 1] Para hacer cuenta regresiva
  (if (== (Variables|Default|GetMinutes) 0)
    (if (== (Variables|Default|GetSeconds) 0)
      (CallFunction|TimeOut)
      (else
        (Utilities|FlowControl|Delay 1.0 :!label _label)
        (Math|Integer|CompareInt (Variables|Default|GetSeconds)
          (:>
            (Math|Integer|DecrementInt (Variables|Default|GetSeconds)
              (:%20%20
                _)))
          (:==
            (Math|Integer|DecrementInt (Variables|Default|GetMinutes)
              (:%20%20
                (Variables|Default|SetSeconds 59)))))
        (Default|ActualizarProgressBar (Variables|Default|GetScoreUI))))
    (else
      (goto _label))))

(event Custom|CalcularTiempoTotal
  ;[1 1 1] Calcular el tiempo total en segundos
  (bind _output_get (Variables|Default|SetTiempoTotal (+ (Variables|Default|GetSeconds) (* (Variables|Default|GetMinutes) 60))))
  (Variables|/Game/Blueprints/Hud_BP.Hud_BP_C|SetIncrementoProgressBar (Variables|Default|GetScoreUI) (/ 1.0 (Math|Conversions|ToFloat(Integer) _output_get))))

(event Custom|TimeOut
  (Variables|Default|SetGameOver? true)
  (Default|DisableHammer (Variables|Default|GetAsHammer_BP))
  (Audio|Components|Audio|Stop (Variables|Default|GetMusic))
  (Utilities|FlowControl|Delay 0.2)
  (Audio|PlaySound2D "/Game/Audios/Finish_Cue.Finish_Cue" 1.0 1.0 0.0 0 0)
  (Variables|/Script/Engine.PlayerController|SetbShowMouseCursor (Game|GetPlayerController 0) true)
  (Audio|PlaySound2D "/Game/Audios/Loading_2__MySims_Cue.Loading_2__MySims_Cue" 1.0 1.0 0.0 0 0)
  (Default|GameOver (Variables|Default|GetScoreUI)))

(event EventBeginPlay
  (Variables|Default|SetGameOver? false)
  (Variables|Default|SetScore 0)
  (Variables|Default|SetPuntaje%20Goodie 300)
  (Variables|Default|SetPuntaje%20Baddie 100)
  (Variables|Default|SetMinutes 0)
  (Variables|Default|SetSeconds 5)
  (Variables|/Script/Engine.PlayerController|SetbShowMouseCursor (Game|GetPlayerController 0) false)
  (bind _returnvalue (UserInterface|CreateWidget "/Game/Blueprints/Hud_BP.Hud_BP_C"))
  (bind _output_get (Variables|Default|SetScoreUI _returnvalue))
  (UserInterface|Viewport|AddtoViewport _output_get 0)
  (CallFunction|CalcularTiempoTotal)
  (bind _returnvalue_2 (AddComponent|AddAudioComponent false))
  (Variables|Default|SetMusic _returnvalue_2)
  (Input|SetInputModeGameOnly (Game|GetPlayerController 0))
  (bind _outactors (Actor|GetAllActorsOfClass "/Game/Blueprints/Hammer_BP.Hammer_BP_C"))
  (Variables|Default|SetAsHammer_BP (Utilities|Array|Get(acopy) _outactors)))

(event EventTick
  (params (DeltaSeconds :type Float%20%28single-precision%29))
  (if (not (Variables|Default|GetGameOver?))
    (CallFunction|CuentaRegresiva)))

(fn ConstructionScript)