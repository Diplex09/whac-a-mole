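; Whack-a-mole mole that repeatedly pops up as a pirate-costumed baddie or, less often, a plain goodie until GameMode_BP reports GameOver.
; A timeline drives its height, alternating hidden and exposed states, with random delays before rising and retreating.
; EventoTopoGolpeado tints it through a dynamic material and lowers it early; the color resets next cycle.
; The logic meant to lower moles at game over is disconnected.
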(event Custom|EventoBajar
  ;[1 1 1] Animación del movimiento del topo
  (bind _z_topo (Timeline|ArribaAbajo ReverseFromEnd)
    (:Update
      (Transformation|SetRelativeLocation (Variables|Default|GetTopo) (Math|Vector|MakeVector 0.0 1e+02 _z_topo) false false))
    (:Finished
      (if (Variables|Default|GetEscondido?)
        (Variables|Default|SetEscondido? false)
        (Variables|Default|SetCollisionable? true)
        (Utilities|FlowControl|Delay (Math|Random|RandomFloatinRange 0.0 1.0))
        (if (Variables|Default|GetCollisionable?)
          (Variables|Default|SetCollisionable? false)
          (CallFunction|EventoBajar))
        (else
          (Variables|Default|SetEscondido? true)
          (CallFunction|EventoSubir))))))

(event Custom|EventoSubir
  (if (not (Variables|/Game/Blueprints/GameMode_BP.GameMode_BP_C|GetGameOver? (Variables|Default|GetAs%20Game%20Mode%20BP)))
    (if (Variables|Default|GetGolpeado?)
      (Variables|Default|SetGolpeado? false)
      (Rendering|Material|SetVectorParameterValue (Variables|Default|GetTopo_Mat) "color" (Variables|Default|GetColor_Topo_Original) :!class /Script/Engine.MaterialInstanceDynamic))
    (Utilities|FlowControl|Delay (Math|Random|RandomFloatinRange 2.0 4.0))
    (Math|Integer|CompareInt (Math|Random|RandomIntegerinRange 1 4) 1
      (:>
        (Variables|Default|SetGoodie? false)
        (CallFunction|GenerarBaddie)
        ;[1 1 1] Animación del movimiento del topo
        (bind _z_topo (Timeline|ArribaAbajo PlayFromStart)
          (:Update
            (Transformation|SetRelativeLocation (Variables|Default|GetTopo) (Math|Vector|MakeVector 0.0 1e+02 _z_topo) false false))
          (:Finished
            (if (Variables|Default|GetEscondido?)
              (Variables|Default|SetEscondido? false)
              (Variables|Default|SetCollisionable? true)
              (Utilities|FlowControl|Delay (Math|Random|RandomFloatinRange 0.0 1.0))
              (if (Variables|Default|GetCollisionable?)
                (Variables|Default|SetCollisionable? false)
                (CallFunction|EventoBajar))
              (else
                (Variables|Default|SetEscondido? true)
                (CallFunction|EventoSubir))))))
      (:==
        (Variables|Default|SetGoodie? true)
        (CallFunction|GenerarGoodie)
        (Timeline|ArribaAbajo PlayFromStart)))))

(event Custom|Evento%20Topo%20Golpeado
  ;[1 1 1] Cuando el martillo coliciona con el topo
  (Variables|Default|SetCollisionable? false)
  (Development|PrintString "Topo golpeado")
  (Rendering|Material|SetVectorParameterValue (Variables|Default|GetTopo_Mat) "color" (Variables|Default|GetColor_Topo_Golpeado) :!class /Script/Engine.MaterialInstanceDynamic)
  (Variables|Default|SetGolpeado? true)
  (CallFunction|EventoBajar))

(event Custom|Generar%20Baddie
  ;[1 1 1] Generar topo goodie o baddie
  (Rendering|SetVisibility (Variables|Default|GetSombrero) true false)
  (Rendering|SetVisibility (Variables|Default|GetCalavera%20de%20sombrero) true false)
  (Rendering|SetVisibility (Variables|Default|GetParche%20de%20ojo) true false)
  (Rendering|SetVisibility (Variables|Default|GetTirante%20de%20parche) true false))

(event Custom|Generar%20Goodie
  ;[1 1 1] Generar topo goodie o baddie
  (Rendering|SetVisibility (Variables|Default|GetSombrero) false false)
  (Rendering|SetVisibility (Variables|Default|GetCalavera%20de%20sombrero) false false)
  (Rendering|SetVisibility (Variables|Default|GetParche%20de%20ojo) false false)
  (Rendering|SetVisibility (Variables|Default|GetTirante%20de%20parche) false false))

(event EventBeginPlay
  (bind _asgame_mode_bp (Utilities|Casting|CastToGameMode_BP (Game|GetGameMode)))
  (Variables|Default|SetAs%20Game%20Mode%20BP _asgame_mode_bp)
  (CallFunction|EventoSubir))

(event EventTick
  (params (DeltaSeconds :type Float%20%28single-precision%29))
  ;[1 1 1] Intento de que todos los topos se bajen juntos al finalizar el tiempo
)

(fn ConstructionScript
  (bind _topo (Variables|Default|GetTopo))
  (bind _returnvalue (Rendering|Material|CreateDynamicMaterialInstance _topo 0 (Rendering|Material|GetMaterial _topo 0) "" :!class /Script/Engine.PrimitiveComponent))
  (bind _output_get (Variables|Default|SetTopo_Mat _returnvalue))
  (Rendering|Material|SetVectorParameterValue _output_get "color" (Variables|Default|GetColor_Topo_Original) :!class /Script/Engine.MaterialInstanceDynamic))