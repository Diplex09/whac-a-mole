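; Player-controlled hammer for a whack-a-mole game, which swings on left click and scores hits on moles (Topo_BP).
; Clicks, throttled by DoOnce and a short delay, play the GolpeMartillo timeline, with a FlipFlop on Finished triggering the return swing.
; Collision overlaps add points, or subtract for goodies, through GameMode_BP, then notify the mole and play a bonk.
; Mouse2D snaps the hammer to the cursor trace at fixed height; DisableHammer disables input and hides it.
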(event OnComponentBeginOverlap(HammerCollision)
  (params (OverlappedComponent :type Primitive%20Component%20Object%20Reference) (OtherActor :type Actor%20Object%20Reference) (OtherComp :type Primitive%20Component%20Object%20Reference) (OtherBodyIndex :type Integer) (bFromSweep :type Boolean) (SweepResult :type Hit%20Result%20Structure%20%28by%20ref%29))
  (bind _as_game_mode_bp (Variables|Default|GetAs%20Game%20Mode%20BP))
  ;[1 1 1] Cuando se golpea un topo
  (bind _astopo_bp (Utilities|Casting|CastToTopo_BP OtherActor))
  (Variables|Default|SetAs%20Topo%20BP _astopo_bp)
  (if (Variables|/Game/Blueprints/Topo_BP.Topo_BP_C|GetCollisionable? (Variables|Default|GetAs%20Topo%20BP))
    (if (Variables|/Game/Blueprints/Topo_BP.Topo_BP_C|GetGoodie? (Variables|Default|GetAs%20Topo%20BP))
      (Default|RestarPuntos _as_game_mode_bp)
      (else
        (Default|SumarPuntos _as_game_mode_bp)))
    (Default|EventoTopoGolpeado (Variables|Default|GetAs%20Topo%20BP))
    (Development|PrintString "Martillo chocó")
    (CallFunction|ReproducirBonk)))

(event Custom|EventoSubir
  ;[1 1 1] Animación de movimiento del martillo
  (bind _x_hammer (Timeline|GolpeMartillo ReverseFromEnd)
    (:Update
      (Transformation|SetRelativeRotation (Variables|Default|GetDefaultSceneRoot) (Math|Rotator|MakeRotator _x_hammer 0.0 0.0) false false))
    (:Finished
      (Utilities|FlowControl|FlipFlop
        (:A
          (CallFunction|EventoSubir))))))

(event Custom|EventoBajar
  ;[1 1 1] Animación de movimiento del martillo
  (bind _x_hammer (Timeline|GolpeMartillo Play)
    (:Update
      (Transformation|SetRelativeRotation (Variables|Default|GetDefaultSceneRoot) (Math|Rotator|MakeRotator _x_hammer 0.0 0.0) false false))
    (:Finished
      (Utilities|FlowControl|FlipFlop
        (:A
          (CallFunction|EventoSubir))))))

(event Custom|DisableHammer
  ;[1 1 1] Disable and remove hammer when game is over
  (Input|DisableInput (Game|GetPlayerController 0))
  (Rendering|SetVisibility (Variables|Default|GetDefaultSceneRoot) false true))

(event Custom|Reproducir%20Bonk
  ;[1 1 1] Hit sound
  (Audio|PlaySound2D "/Game/Audios/Bonk_Cue.Bonk_Cue" 1.0 1.0 0.0 0 0))

(event EventBeginPlay
  (bind _asgame_mode_bp (Utilities|Casting|CastToGameMode_BP (Game|GetGameMode)))
  (Variables|Default|SetAs%20Game%20Mode%20BP _asgame_mode_bp))

(event Input|MouseEvents|LeftMouseButton
  (params (Key :type Key%20Structure :default "None"))
  ;[1 1 1] Cuando el jugador hace clic
  (:Pressed
    (Utilities|FlowControl|DoOnce false :!label _label
      (:Completed
        (CallFunction|EventoBajar)
        (Utilities|FlowControl|Delay 0.3)
        (goto _label Reset)))))

(event Input|MouseEvents|Mouse2D
  (params (AxisValue :type Vector :default "0, 0, 0"))
  (bind _returnvalue (Class|GameplayStatics|GetPlayerControllerfromID))
  (bind _object_types (Variables|Default|GetObject%20Types))
  (bind _hitresult (Class|PlayerController|GetHitResultUnderCursorforObjects _returnvalue _object_types true))
  (bind _location (Collision|BreakHitResult _hitresult))
  (bind (_x _y) (Math|Vector|BreakVector _location))
  (Transformation|SetActorLocation (Math|Vector|MakeVector _x _y 1.1e+02) false false))

(fn ConstructionScript)